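; Player Blueprint that moves and turns its actor from the Moveforward, Moveright and Spinyaw input values.
; Each Tick scales these values by delta time and the Linervel or Angularvel speed, then applies them as a local transform offset for forward, sideways and yaw motion.
; BeginPlay, overlap and construction graphs are empty.
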(event EventBeginPlay)

(event Collision|EventActorBeginOverlap
  (params (OtherActor :type Actor%20Object%20Reference)))

(event EventTick
  (params (DeltaSeconds :type Float%20%28single-precision%29))
  (bind _linervel (Variables|Default|Getlinervel))
  (bind _returnvalue (* DeltaSeconds _linervel))
  (Class|Actor|AddActorLocalTransform (Math|Transform|MakeTransform (Math|Vector|MakeVector (* _returnvalue (Input|AxisValues|Getmoveforward)) (* _returnvalue (Input|AxisValues|Getmoveright)) 0.0) (Math|Rotator|MakeRotator 0.0 0.0 (* (* DeltaSeconds (Variables|Default|Getangularvel)) (Input|AxisValues|Getspinyaw))) "1,1,1") false false))

(fn ConstructionScript)