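; Player Blueprint that moves and turns the player in its own local space.
; Each Tick, math expression nodes multiply linear or angular velocity by delta seconds and the MoveForward, MoveRight and SpinYaw values for frame-rate-independent motion.
; The results feed a single AddActorLocalTransform as X and Y translation and yaw rotation.
; BeginPlay, overlap and construction script are empty.
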(event EventBeginPlay)

(event Collision|EventActorBeginOverlap
  (params (OtherActor :type Actor%20Object%20Reference)))

(event EventTick
  (params (DeltaSeconds :type Float%20%28single-precision%29))
  (Class|Actor|AddActorLocalTransform (Math|Transform|MakeTransform (Math|Vector|MakeVector (|(({F558DAD7-406F-8194-440E-5CA5AA569767}*deltaTime)*moveForward) (Utilities|Time|GetWorldDeltaSeconds) (Input|AxisValues|Getmoveforward)) (|((linervel*deltaTime)*moveRight) (Utilities|Time|GetWorldDeltaSeconds) (Input|AxisValues|Getmoveright)) 0.0) (Math|Rotator|MakeRotator 0.0 0.0 (|((angularvel*deltaTime)*spinYaw) (Utilities|Time|GetWorldDeltaSeconds) (Input|AxisValues|Getspinyaw))) "1,1,1") false false))

(fn ConstructionScript)